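; AI character Blueprint for the Sidhe Rigel hero that highlights itself when the mouse cursor hovers over it.
; On BeginPlay it caches its skeletal mesh component and, if that component is valid, binds the cursor-over begin and end events.
; Those handlers toggle custom depth rendering on the Mesh component, while the construction script stays empty.
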(event Custom|OnMouseHover
  (params (TouchedActor :type Actor%20Object%20Reference))
  (Rendering|SetRenderCustomDepth (Variables|Character|GetMesh) true))

(event Custom|OnMouseHoverEnd
  (params (TouchedActor :type Actor%20Object%20Reference))
  (Rendering|SetRenderCustomDepth (Variables|Character|GetMesh) false))

(event EventBeginPlay
  (bind _self self)
  (bind _returnvalue (Actor|GetComponentbyClass _self "/Script/Engine.SkeletalMeshComponent"))
  (Utilities|IsValid _returnvalue
    (:Is%20Valid
      (Variables|Default|SetCharacterMeshRef _returnvalue)
      (EventDispatchers|BindEventtoOnBeginCursorOver _self (delegate Custom|OnMouseHover))
      (EventDispatchers|BindEventtoOnEndCursorOver _self (delegate Custom|OnMouseHoverEnd)))))

(event Collision|EventActorBeginOverlap
  (params (OtherActor :type Actor%20Object%20Reference)))

(event EventTick
  (params (DeltaSeconds :type Float%20%28single-precision%29)))

(fn ConstructionScript)